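; BP_Enemy is an enemy actor that moves onto the BP_GridManager tile in front of it, starting after a delay at BeginPlay.
; FUMoveTO box-traces ahead of the Body and reads the hit tile's world location from the grid's instanced mesh using the hit item index.
; The MoveTO timeline lerps Scene from its current location toward that point in X and Y, keeping its height.
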(event Custom|Tick
  (bind _scene (Variables|Default|GetScene))
  (bind _returnvalue (Transformation|GetWorldLocation _scene))
  (bind _out_instance_transform_location (CallFunction|FUMoveTO))
  (Variables|Default|SetOut%20Instance%20Transform%20Location _out_instance_transform_location)
  (bind _aimoveto (Timeline|Move%20TO PlayFromStart)
    (:Update
      (Transformation|SetWorldLocation (Variables|Default|GetScene) (Math|Vector|MakeVector (.x (Math|Vector|Lerp(Vector) (Math|Vector|MakeVector (.x _returnvalue) (.y _returnvalue) (.z _returnvalue)) (Variables|Default|GetOut%20Instance%20Transform%20Location) _aimoveto)) (.y (Math|Vector|Lerp(Vector) (Math|Vector|MakeVector (.x _returnvalue) (.y _returnvalue) (.z _returnvalue)) (Variables|Default|GetOut%20Instance%20Transform%20Location) _aimoveto)) (.z _returnvalue)) false false))))

(event EventBeginPlay
  (Utilities|FlowControl|Delay 5.0)
  (CallFunction|Tick))

(event Collision|EventActorBeginOverlap
  (params (OtherActor :type Actor%20Object%20Reference)))

(event EventTick
  (params (DeltaSeconds :type Float%20%28single-precision%29)))

(fn ConstructionScript)

(fn FUMoveTO
  (bind _body (Variables|Default|GetBody))
  (bind _returnvalue (Transformation|GetWorldLocation _body))
  (bind _returnvalue_2 (Math|Vector|GetForwardVector _body))
  (bind _returnvalue_3 (* _returnvalue_2 100))
  (bind _returnvalue_4 (+ _returnvalue _returnvalue_3))
  (bind _outhit (Class|KismetSystemLibrary|BoxTraceSingleforObjects _returnvalue_4 _returnvalue_4 "50.000000,50.000000,50.000000" (Transformation|GetWorldRotation _body) (Utilities|Array|MakeArray "ObjectTypeQuery2") false 0 "ForOneFrame" true))
  (bind _asbp_grid_manager (Utilities|Casting|CastToBP_GridManager (.HitActor (Collision|BreakHitResult _outhit))))
  (return (.location (.OutInstanceTransform (Components|InstancedStaticMesh|GetInstanceTransform (Variables|/Game/Map/BluePrint/BP_GridManager.BP_GridManager_C|GetHierarchicalInstancedStaticMesh _asbp_grid_manager) (.HitItem (Collision|BreakHitResult _outhit)) true)))))